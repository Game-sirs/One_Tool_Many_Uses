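; BP_Stump is a stump actor that can latch onto BP_MainCharacter's ShtoporSocket.
; A sphere overlap stores the character and starts a looping timer that checks its state.
; In the matching state, if nothing is attached, it sets the Attach flag, attaches to the socket, disables Stump collision and snaps the root to the socket.
; Any other state clears the stored reference; the start location is saved but unused here.
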(event OnComponentBeginOverlap(Sphere)
  (params (OverlappedComponent :type Primitive%20Component%20Object%20Reference) (OtherActor :type Actor%20Object%20Reference) (OtherComp :type Primitive%20Component%20Object%20Reference) (OtherBodyIndex :type Integer) (bFromSweep :type Boolean) (SweepResult :type Hit%20Result%20Structure%20%28by%20ref%29))
  (bind _asbp_main_character (Utilities|Casting|CastToBP_MainCharacter OtherActor))
  (Variables|Default|SetAs%20BP%20Main%20Character _asbp_main_character)
  (Utilities|Time|SetTimerbyEvent (delegate Custom|CustomEvent) 0.2 true))

(event Custom|CustomEvent
  (bind _defaultsceneroot (Variables|Default|GetDefaultSceneRoot))
  (Utilities|IsValid (Variables|Default|GetAs%20BP%20Main%20Character)
    (:Is%20Valid
      (if (Utilities|Enum|Equal(Enum) (Variables|/Game/MainGame/Core/BP_MainCharacter.BP_MainCharacter_C|GetStateIndex (stale OnComponentBeginOverlap(Sphere) _asbp_main_character)) "NewEnumerator2")
        (if (not (Variables|/Game/MainGame/Core/BP_MainCharacter.BP_MainCharacter_C|GetAttach? (stale OnComponentBeginOverlap(Sphere) _asbp_main_character)))
          (Variables|/Game/MainGame/Core/BP_MainCharacter.BP_MainCharacter_C|SetAttach? (stale OnComponentBeginOverlap(Sphere) _asbp_main_character) true)
          (Transformation|AttachComponentToComponent (Variables|/Script/Engine.Character|GetMesh (stale OnComponentBeginOverlap(Sphere) _asbp_main_character)) "ShtoporSocket" "KeepWorld" "KeepWorld" "KeepWorld" false)
          (Collision|SetCollisionEnabled (Variables|Default|GetStump) "NoCollision")
          (Transformation|SetWorldLocation _defaultsceneroot (Transformation|GetSocketLocation (Variables|/Script/Engine.Character|GetMesh (stale OnComponentBeginOverlap(Sphere) _asbp_main_character)) "ShtoporSocket") false false)
          (Transformation|SetWorldRotation _defaultsceneroot (Transformation|GetSocketRotation (Variables|/Script/Engine.Character|GetMesh (stale OnComponentBeginOverlap(Sphere) _asbp_main_character)) "ShtoporSocket") false false))
        (else
          (Variables|Default|SetAs%20BP%20Main%20Character 0))))))

(event EventBeginPlay
  (Variables|Default|SetOriginTransform (Transformation|GetWorldLocation (Variables|Default|GetStump))))

(event Collision|EventActorBeginOverlap
  (params (OtherActor :type Actor%20Object%20Reference)))

(event EventTick
  (params (DeltaSeconds :type Float%20%28single-precision%29)))

(event EventDestroyed)

(fn ConstructionScript)