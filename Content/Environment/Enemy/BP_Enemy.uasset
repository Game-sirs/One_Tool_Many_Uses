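; BP_Enemy is a rat-like enemy that creeps toward the player and kills the player character when it overlaps the enemy's DamageColl.
; Tick switches on RunHome between a slow move to PlayerRef and a fast retreat to RatHome, captured from the actor location in the construction script.
; Capsule overlap with a component named "knife" sets RunHome.
; Any end overlap clears it, as that check compares OtherComp to itself.
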(event OnComponentBeginOverlap(CapsuleComponent)
  (params (OverlappedComponent :type Primitive%20Component%20Object%20Reference) (OtherActor :type Actor%20Object%20Reference) (OtherComp :type Primitive%20Component%20Object%20Reference) (OtherBodyIndex :type Integer) (bFromSweep :type Boolean) (SweepResult :type Hit%20Result%20Structure%20%28by%20ref%29))
  (Variables|Default|SetRunHome (Utilities|Enum|Equal(Enum) (Utilities|GetObjectName OtherComp) "knife")))

(event OnComponentEndOverlap(CapsuleComponent)
  (params (OverlappedComponent :type Primitive%20Component%20Object%20Reference) (OtherActor :type Actor%20Object%20Reference) (OtherComp :type Primitive%20Component%20Object%20Reference) (OtherBodyIndex :type Integer))
  (if (== (stale OnComponentBeginOverlap(CapsuleComponent) OtherComp) OtherComp)
    (Variables|Default|SetRunHome false)))

(event OnComponentBeginOverlap(damageColl)
  (params (OverlappedComponent :type Primitive%20Component%20Object%20Reference) (OtherActor :type Actor%20Object%20Reference) (OtherComp :type Primitive%20Component%20Object%20Reference) (OtherBodyIndex :type Integer) (bFromSweep :type Boolean) (SweepResult :type Hit%20Result%20Structure%20%28by%20ref%29))
  (if (== (Utilities|GetClass OtherActor) "/Game/MainGame/Core/BP_MainCharacter.BP_MainCharacter_C")
    (Default|Death (Utilities|ResolveSoftReference (Variables|Default|GetPlayerRef)))))

(event EventTick
  (params (DeltaSeconds :type Float%20%28single-precision%29))
  (bind _self self)
  (bind _returnvalue (AI|GetAIController _self))
  (if (Variables|Default|GetRunHome)
    (AI|Navigation|SimpleMovetoLocation _returnvalue (Variables|Default|GetRatHome))
    (Variables|/Script/Engine.CharacterMovementComponent|SetMaxWalkSpeed (Variables|Character|GetCharacterMovement) 6e+02) ; убегает со всех ног
    (else
      (AI|Navigation|SimpleMovetoActor _returnvalue (Utilities|ResolveSoftReference (Variables|Default|GetPlayerRef)))
      (Variables|/Script/Engine.CharacterMovementComponent|SetMaxWalkSpeed (Variables|Character|GetCharacterMovement) 1e+02) ; побаивается
    )))

(event EventBeginPlay)

(fn ConstructionScript
  (Variables|Default|SetRatHome (Transformation|GetActorLocation)))