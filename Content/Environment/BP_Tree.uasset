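; BP_Tree is an environment tree actor that leaves a BP_Stump at its location when destroyed.
; The construction script uses the clamped Index to pick one of three tree meshes and scale the test collision box to match.
; As a respawn test, BP_MainCharacter overlapping that box with a matching StateIndex destroys the tree after a one-second delay.
; The stump spawn sits in the Destroyed event, so it is independent of that test trigger.
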(event OnComponentBeginOverlap(BoxCollisionTest)
  (params (OverlappedComponent :type Primitive%20Component%20Object%20Reference) (OtherActor :type Actor%20Object%20Reference) (OtherComp :type Primitive%20Component%20Object%20Reference) (OtherBodyIndex :type Integer) (bFromSweep :type Boolean) (SweepResult :type Hit%20Result%20Structure%20%28by%20ref%29))
  ;[1 1 1] Для теста респана актора
  (bind _asbp_main_character (Utilities|Casting|CastToBP_MainCharacter OtherActor))
  (if (Utilities|Enum|Equal(Enum) (Variables|/Game/MainGame/Core/BP_MainCharacter.BP_MainCharacter_C|GetStateIndex _asbp_main_character) (Variables|Default|GetValidState))
    (Development|PrintString (Utilities|String|Append "State is" (Utilities|String|EnumtoString (Variables|/Game/MainGame/Core/BP_MainCharacter.BP_MainCharacter_C|GetStateIndex _asbp_main_character))))
    (if (== (Utilities|GetClass OtherActor) "/Game/MainGame/Core/BP_MainCharacter.BP_MainCharacter_C")
      (Utilities|FlowControl|Delay 1.0)
      (Actor|DestroyActor))
    (else
      (Development|PrintString "Not valid state"))))

(event EventBeginPlay)

(event EventDestroyed
  (|CallParentFunction)
  (Game|SpawnActorfromClass "/Game/Environment/BP_Stump.BP_Stump_C" (Math|Transform|MakeTransform (Transformation|GetWorldLocation (Variables|Default|GetDefaultSceneRoot)) "0, 0, 0" "1.000000,1.000000,1.000000") "AdjustIfPossibleButAlwaysSpawn" "MultiplyWithRoot" 0 0))

(fn ConstructionScript
  (|CallParentFunction)
  (Components|StaticMesh|SetStaticMesh (Variables|Default|GetStaticMesh) (Utilities|Select :Index (Math|Integer|Clamp(Integer) (Variables|Default|GetIndex) 0 2) :Option%200 "/Game/Environment/Props/derevo_1.derevo_1" :Option%201 "/Game/Environment/Props/derevo_2.derevo_2" :Option%202 "/Game/Environment/Props/derevo_3.derevo_3"))
  (Transformation|SetRelativeScale3D (Variables|Default|GetBoxCollisionTest) (Utilities|Select :Index (Math|Integer|Clamp(Integer) (Variables|Default|GetIndex) 0 2) :Option%200 "8.000000,8.000000,2.000000" :Option%201 "6.000000,6.000000,2.000000" :Option%202 "4.000000,4.000000,2.000000")))