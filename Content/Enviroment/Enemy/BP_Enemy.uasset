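; Enemy Blueprint that uses its AI controller to move toward either the player or RatHome.
; Tick reissues a simple move-to-actor request, choosing the goal from a FlipFlop's state.
; BeginPlay triggers that FlipFlop once after a short delay, switching the goal to the player, and nothing in the graph flips it back.
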(event EventBeginPlay
  (bind _self self)
  (bind _returnvalue (AI|GetAIController _self))
  (Utilities|FlowControl|Delay 5.0)
  (bind _isa (Utilities|FlowControl|FlipFlop)
    (:A
      (if _isa
        (AI|Navigation|SimpleMovetoActor _returnvalue (Utilities|ResolveSoftReference (Variables|Default|GetPlayerRef)))
        (else
          (AI|Navigation|SimpleMovetoActor _returnvalue (Variables|Default|GetRatHome)))))))

(event EventTick
  (params (DeltaSeconds :type Float%20%28single-precision%29))
  (bind _self self)
  (bind _returnvalue (AI|GetAIController _self))
  (if (stale EventBeginPlay _isa)
    (AI|Navigation|SimpleMovetoActor _returnvalue (Utilities|ResolveSoftReference (Variables|Default|GetPlayerRef)))
    (else
      (AI|Navigation|SimpleMovetoActor _returnvalue (Variables|Default|GetRatHome)))))

(fn ConstructionScript)