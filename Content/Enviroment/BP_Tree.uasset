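; BP_Tree is an environment tree actor whose overlap logic is marked as a test for actor respawn.
; When BP_MainCharacter overlaps its test box and the character's StateIndex matches ValidState, it prints the state and destroys itself after a short delay.
; A mismatched state only prints a debug message.
; Destroyed defers to the parent class, and no respawn logic appears in this Blueprint itself.
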(event OnComponentBeginOverlap(BoxCollisionTest)
  (params (OverlappedComponent :type Primitive%20Component%20Object%20Reference) (OtherActor :type Actor%20Object%20Reference) (OtherComp :type Primitive%20Component%20Object%20Reference) (OtherBodyIndex :type Integer) (bFromSweep :type Boolean) (SweepResult :type Hit%20Result%20Structure%20%28by%20ref%29))
  ;[1 1 1] Для теста респана актора
  (bind _asbp_main_character (Utilities|Casting|CastToBP_MainCharacter OtherActor))
  (if (Utilities|Enum|Equal(Enum) (Variables|/Game/MainGame/Core/BP_MainCharacter.BP_MainCharacter_C|GetStateIndex _asbp_main_character) (Variables|Default|GetValidState))
    (Development|PrintString (Utilities|String|Append "State is" (Utilities|String|EnumtoString (Variables|/Game/MainGame/Core/BP_MainCharacter.BP_MainCharacter_C|GetStateIndex _asbp_main_character))))
    (if (== (Utilities|GetClass OtherActor) "/Game/MainGame/Core/BP_MainCharacter.BP_MainCharacter_C")
      (Utilities|FlowControl|Delay 1.0)
      (Actor|DestroyActor))
    (else
      (Development|PrintString "Not valid state"))))

(event Collision|EventActorBeginOverlap
  (params (OtherActor :type Actor%20Object%20Reference)))

(event EventTick
  (params (DeltaSeconds :type Float%20%28single-precision%29)))

(event EventDestroyed
  (|CallParentFunction))

(fn ConstructionScript
  (|CallParentFunction))